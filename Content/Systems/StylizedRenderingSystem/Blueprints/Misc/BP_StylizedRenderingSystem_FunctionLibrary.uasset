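; Blueprint function library of shared helpers for the Stylized Rendering System.
; Light color registration and unregistration by ID are forwarded to a light color manager obtained through a message to the Game State.
; SetBoundsParameters writes an actor's location, axes and scaled primary and secondary bounds to a material as oriented-bounds parameters.
; Vector alpha channels pack feathering and a signed secondary-bounds mode: inside, outside or disabled.
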(fn GetLightManager
  (bind _light_color_manager (Class|BPCelShadedLightManagerInterface|GetLightColorManager(Message) (Game|GetGameState)))
  (return _light_color_manager))

(fn RegisterLightColor
  (params (Color :type Linear%20Color%20Structure))
  (bind _id (Default|RegisterLightColor (CallFunction|GetLightManager) Color))
  (return _id))

(fn UnregisterLightColor
  (params (ID :type Integer%20%28by%20ref%29))
  (bind _successful (Default|UnregisterLightColor (CallFunction|GetLightManager) ID))
  (return _successful))

(fn SetBoundsParameters
  (params (Target%20Material :type Material%20Instance%20Dynamic%20Object%20Reference) (Actor :type Actor%20Object%20Reference) (Enable%20Primary%20Bounds :type Boolean) (Primary%20Bounds%20Scale :type Vector) (Primary%20Bounds%20Feathering :type Float%20%28single-precision%29) (Secondary%20Bounds%20Behaviour :type BP_SRS_BoundsBehaviour%20Enum :default "NewEnumerator0") (Enable%20Secondary%20Bounds :type Boolean) (Secondary%20Bounds%20Size :type Vector) (Secondary%20Bounds%20Feathering :type Float%20%28single-precision%29))
  (bind _returnvalue (Transformation|GetActorScale3D Actor))
  (bind _returnvalue_2 (Transformation|GetActorLocation Actor))
  (bind _returnvalue_3 (Transformation|GetActorScale3D Actor))
  (bind _returnvalue_4 (* Secondary%20Bounds%20Size _returnvalue_3))
  (bind _returnvalue_5 (* Primary%20Bounds%20Scale _returnvalue))
  (Rendering|Material|SetVectorParameterValue Target%20Material "Bounds Origin" (Math|Color|MakeColor (.x _returnvalue_2) (.y _returnvalue_2) (.z _returnvalue_2) (select Enable%20Secondary%20Bounds (Utilities|Select :Index Secondary%20Bounds%20Behaviour :NewEnumerator0 1.0 :NewEnumerator3 -1.0) 0.0)) :!class /Script/Engine.MaterialInstanceDynamic)
  (Rendering|Material|SetVectorParameterValue Target%20Material "Bounds Size" (Math|Color|MakeColor (.x _returnvalue_4) (.y _returnvalue_4) (.z _returnvalue_4) Secondary%20Bounds%20Feathering) :!class /Script/Engine.MaterialInstanceDynamic)
  (Rendering|Material|SetVectorParameterValue Target%20Material "Bounds Forward Vector" (Math|Conversions|ToLinearColor(Vector) (Math|Vector|Normalize (Transformation|GetActorForwardVector Actor))) :!class /Script/Engine.MaterialInstanceDynamic)
  (Rendering|Material|SetVectorParameterValue Target%20Material "Bounds Right Vector" (Math|Conversions|ToLinearColor(Vector) (Math|Vector|Normalize (Transformation|GetActorRightVector Actor))) :!class /Script/Engine.MaterialInstanceDynamic)
  (Rendering|Material|SetVectorParameterValue Target%20Material "Bounds Up Vector" (Math|Conversions|ToLinearColor(Vector) (Math|Vector|Normalize (Transformation|GetActorUpVector Actor))) :!class /Script/Engine.MaterialInstanceDynamic)
  (Rendering|Material|SetVectorParameterValue Target%20Material "Primary Bounds Size" (Utilities|Struct|MakeLinearColor (.x _returnvalue_5) (.y _returnvalue_5) (.z _returnvalue_5) Primary%20Bounds%20Feathering) :!class /Script/Engine.MaterialInstanceDynamic)
  (Rendering|Material|SetScalarParameterValue Target%20Material "Enable Primary Bounds Feathering" (Math|Conversions|ToFloat(Boolean) (and (!= Primary%20Bounds%20Feathering 0.0) Enable%20Primary%20Bounds)) :!class /Script/Engine.MaterialInstanceDynamic))