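; Test character that moves along world X and Y with hardcoded WASD key events.
; The keys set X and Y values, which Tick normalizes and feeds straight into CharacterMovement as an input vector.
; Releasing either key of a pair zeroes that axis, even if the opposite key is still held.
; On BeginPlay it caches the level's GridManager and prints a debug message if valid, but does not otherwise use it.
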(event EventBeginPlay
  (bind _returnvalue (Actor|GetActorOfClass "/Script/ProjectISG.GridManager"))
  (bind _output_get (Variables|Default|SetGridManager _returnvalue))
  (Utilities|IsValid _output_get
    (:Is%20Valid
      (Development|PrintString "Manager Valid"))))

(event EventTick
  (params (DeltaSeconds :type Float%20%28single-precision%29))
  (Class|PawnMovementComponent|AddInputVector (Variables|Character|GetCharacterMovement) (Math|Vector|Normalize (Math|Vector|MakeVector (Variables|Default|GetX) (Variables|Default|GetY) 0.0)) false))

(event Input|KeyboardEvents|S
  (params (Key :type Key%20Structure :default "None"))
  (:Pressed
    (Variables|Default|SetX -1.0))
  (:Released
    (Variables|Default|SetX 0.0)))

(event Input|KeyboardEvents|W
  (params (Key :type Key%20Structure :default "None"))
  (:Pressed
    (Variables|Default|SetX 1.0))
  (:Released
    (Variables|Default|SetX 0.0)))

(event Input|KeyboardEvents|A
  (params (Key :type Key%20Structure :default "None"))
  (:Pressed
    (Variables|Default|SetY -1.0))
  (:Released
    (Variables|Default|SetY 0.0)))

(event Input|KeyboardEvents|D
  (params (Key :type Key%20Structure :default "None"))
  (:Pressed
    (Variables|Default|SetY 1.0))
  (:Released
    (Variables|Default|SetY 0.0)))

(fn ConstructionScript)