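; Trigger actor that moves the player from the TrainStation streaming level into PlayLevel when MainPlayerCharacter overlaps its Root component.
; The overlap loads PlayLevel with blocking, then searches all PlayerStart actors for those belonging to that loaded level.
; For each match, it teleports player 0's pawn to that location without sweep and requests a non-blocking unload of TrainStation.
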(event OnComponentBeginOverlap(Root)
  (params (OverlappedComponent :type Primitive%20Component%20Object%20Reference) (OtherActor :type Actor%20Object%20Reference) (OtherComp :type Primitive%20Component%20Object%20Reference) (OtherBodyIndex :type Integer) (bFromSweep :type Boolean) (SweepResult :type Hit%20Result%20Structure%20%28by%20ref%29))
  (Utilities|Casting|CastToMainPlayerCharacter OtherActor)
  (Game|LoadStreamLevel(byName) "PlayLevel" true true)
  (bind _outactors (Actor|GetAllActorsOfClass "/Script/Engine.PlayerStart"))
  (for _array_element _outactors
    (if (== (Class|Actor|GetLevel _array_element) (Class|LevelStreaming|GetLoadedLevel (Class|GameplayStatics|GetStreamingLevel "PlayLevel")))
      (Transformation|SetActorLocation (Game|Player|GetPlayerPawn 0) (Transformation|GetActorLocation _array_element) false true)
      (Game|UnloadStreamLevel(byName) "TrainStation" false))))

(event EventBeginPlay)

(event Collision|EventActorBeginOverlap
  (params (OtherActor :type Actor%20Object%20Reference)))

(event EventTick
  (params (DeltaSeconds :type Float%20%28single-precision%29)))

(fn ConstructionScript)